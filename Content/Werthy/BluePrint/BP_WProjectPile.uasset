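; BP_WProjectPile is a projectile actor that scores target hits and knocks physics objects around.
; On hit it only reacts to components simulating physics.
; A hit on an actor tagged Target adds a point to the owning BP_WCharacter's Score, without an impulse or destroying the projectile.
; Any other physics hit applies a velocity-scaled impulse at the projectile's location, then destroys it.
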(event Collision|EventHit
  (params (MyComp :type Primitive%20Component%20Object%20Reference) (Other :type Actor%20Object%20Reference) (OtherComp :type Primitive%20Component%20Object%20Reference) (bSelfMoved :type Boolean) (HitLocation :type Vector :default "0, 0, 0") (HitNormal :type Vector :default "0, 0, 0") (NormalImpulse :type Vector :default "0, 0, 0") (Hit :type Hit%20Result%20Structure%20%28by%20ref%29))
  (if (Physics|IsSimulatingPhysics OtherComp "None")
    (if (Actor|ActorHasTag Other "Target")
      (bind _asbp_wcharacter (Utilities|Casting|CastToBP_WCharacter (Components|GetOwner))
        (:then
          (Variables|/Game/Werthy/BluePrint/BP_WCharacter.BP_WCharacter_C|SetScore _asbp_wcharacter (+ (Variables|/Game/Werthy/BluePrint/BP_WCharacter.BP_WCharacter_C|GetScore _asbp_wcharacter) 1)))
        (:CastFailed
          (Development|PrintString "Failed")))
      (else
        (Physics|AddImpulseatLocation OtherComp (* (Transformation|GetVelocity) 1e+02) (Transformation|GetActorLocation) "None")
        (Actor|DestroyActor) ; Then destroy this projectile
      ))))

(fn ConstructionScript
  (|CallParentFunction))